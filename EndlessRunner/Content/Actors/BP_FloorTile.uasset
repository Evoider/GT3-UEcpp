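; Floor tile actor that exposes an attach transform for chaining tiles, as in an endless runner.
; Construction script rolls a weighted chance to add either one random obstacle or a random number of pickups.
; These are child actor components with random classes, placed at random points within the ObstacleZone or CoinArea box.
; Any overlap with ExitTile fires the OnExitTile dispatcher, then destroys the tile after a short delay.
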(event `self.ReceiveBeginPlay`)

(event `self.ExitTile.OnComponentBeginOverlap`
  (params (OverlappedComponent :type "PrimitiveComponent Object Reference") (OtherActor :type "Actor Object Reference") (OtherComp :type "PrimitiveComponent Object Reference") (OtherBodyIndex :type Integer) (bFromSweep :type Boolean) (SweepResult :type "HitResult Structure (by ref)"))
  (`self.OnExitTile` self)
  (`KismetSystemLibrary.Delay` 2.0)
  (`self.K2_DestroyActor`))

(fn `GetAttachTransform`
  (returns (AttachPoint :type "Transform Structure"))
  (return (`SceneComponent.K2_GetComponentToWorld` (`self.AttachPoint`))))

(fn `SpawnCoins`
  (params (`Max Number of coins` :type Integer))
  (bind _coinarea (`self.CoinArea`))
  (for _ (range (`KismetMathLibrary.RandomInteger` `Max Number of coins`) (+ `Max Number of coins` 1))
    (bind _returnvalue (`AddComponent|NODE_AddChildActorComponent-6` :`RelativeTransform` (`KismetMathLibrary.Conv_VectorToTransform` (`KismetMathLibrary.RandomPointInBoundingBox` (`SceneComponent.RelativeLocation` _coinarea) (`BoxComponent.BoxExtent` _coinarea)))))
    (`ChildActorComponent.SetChildActorClass` _returnvalue (`KismetArrayLibrary.Array_Random` (`self.Pickups`)))))

(fn `SpawnObstacle`
  (returns (ObstacleSpawned :type "/Game/Actors/BP_Obstacle Object Reference"))
  (bind _obstaclezone (`self.ObstacleZone`))
  (bind _returnvalue (`AddComponent|NODE_AddChildActorComponent-7` :`RelativeTransform` (`KismetMathLibrary.Conv_VectorToTransform` (`KismetMathLibrary.RandomPointInBoundingBox` (`SceneComponent.RelativeLocation` _obstaclezone) (`BoxComponent.BoxExtent` _obstaclezone)))))
  (`ChildActorComponent.SetChildActorClass` _returnvalue (`KismetArrayLibrary.Array_Random` (`self.Obstacle`)))
  (return null))

(fn `UserConstructionScript`
  (if (`KismetMathLibrary.RandomBoolWithWeight` (`self.%ChancesOfObstacles`))
    (`self.SpawnObstacle`)
    (else
      (`self.SpawnCoins` (`self.MaxNumberOfCoins`)))))