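; BP_RunCharacter is the player character for a running game, speeding up over time and tracking coins and death.
; Tick steadily raises max walk speed and, while alive, converts velocity to whole km/h.
; Die fires once: it ragdolls the mesh, stops the run controller's running and input, spawns explosion effects, and calls OnPlayerDie.
; AddCoin increases the total, while RemoveCoin sets it to Amount minus TotalCoins, an apparently reversed subtraction.
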(event `self.ReceiveBeginPlay`
  (bind _asbp_pc_run_character (cast `/Game/Controllers/BP_PC_RunCharacter` (`GameplayStatics.GetPlayerController` 0)))
  (set `self.RunController` _asbp_pc_run_character))

(event `Die`
  (bind _returnvalue (`self.K2_GetActorLocation`))
  (bind _mesh (`self.Mesh`))
  (if (not (`self.IsDead`))
    (`PrimitiveComponent.SetSimulatePhysics` _mesh true)
    (`PrimitiveComponent.SetCollisionEnabled` _mesh "PhysicsOnly")
    (set `/Game/Controllers/BP_PC_RunCharacter.CanRun` false (`self.RunController`))
    (`self.DisableInput` (`self.RunController`) null)
    (`GameplayStatics.SpawnEmitterAtLocation` "/Game/Ressources/StarterContent/Particles/P_Explosion.P_Explosion" _returnvalue (struct) (3.0 3.0 3.0))
    (`GameplayStatics.SpawnSoundAtLocation` "/Game/Ressources/StarterContent/Audio/Explosion_Cue.Explosion_Cue" _returnvalue (struct) 1.0 1.0 0.0 null null)
    (set `self.IsDead` true)
    (`self.OnPlayerDie`)))

(event `self.ReceiveTick`
  (params (DeltaSeconds :type "Float (single-precision)"))
  (bind _charactermovement (`self.CharacterMovement`))
  (set `CharacterMovementComponent.MaxWalkSpeed` (+ (* DeltaSeconds (`self.Speed`)) (`CharacterMovementComponent.MaxWalkSpeed` _charactermovement)) _charactermovement)
  (if (not (`self.IsDead`))
    (set `self.CurrentSpeed` (`KismetMathLibrary.FTrunc` (* (`KismetMathLibrary.VSize` (`self.GetVelocity`)) 0.036)))))

(fn `AddCoin`
  (params (Amount :type Integer))
  (set `self.TotalCoins` (+ Amount (`self.TotalCoins`)))
  (return))

(fn `RemoveCoin`
  (params (Amount :type Integer))
  (set `self.TotalCoins` (- Amount (`self.TotalCoins`))))

(fn `UserConstructionScript`)