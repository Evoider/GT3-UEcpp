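; BP_PickupItem is a pickup actor that the player character collects by touching its static mesh.
; On overlap with player 0's BP_RunCharacter, it stores that character as Player, calls OnHit and destroys itself.
; OnHit plays an optional sound and spawns a scaled-down steam particle effect just above the pickup, and grants nothing itself.
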(event `self.StaticMesh.OnComponentBeginOverlap`
  (params (OverlappedComponent :type "PrimitiveComponent Object Reference") (OtherActor :type "Actor Object Reference") (OtherComp :type "PrimitiveComponent Object Reference") (OtherBodyIndex :type Integer) (bFromSweep :type Boolean) (SweepResult :type "HitResult Structure (by ref)"))
  (if (== OtherActor (`GameplayStatics.GetPlayerCharacter` 0))
    (bind _asbp_run_character (cast `/Game/Actors/BP_RunCharacter` OtherActor))
    (set `self.Player` _asbp_run_character)
    (`self.OnHit`)
    (`self.K2_DestroyActor`)))

(fn `OnHit`
  (bind _returnvalue (`self.K2_GetActorLocation`))
  (bind _sound (`self.Sound`)
    (:`then`
      (`GameplayStatics.SpawnSoundAtLocation` _sound _returnvalue (struct) 1.0 1.0 0.0 null null))
    (:`else`
      _))
  (`GameplayStatics.SpawnEmitterAtLocation` "/Game/Ressources/StarterContent/Particles/P_Steam_Lit.P_Steam_Lit" (+ _returnvalue (0.0 0.0 50.0)) (struct) (0.5 0.5 0.5))
  (return))

(fn `UserConstructionScript`)