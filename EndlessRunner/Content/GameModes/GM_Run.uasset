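; Game mode for a tile-based runner that builds the floor path, shows the player HUD and restarts the level after death.
; BeginPlay binds to the run character's death event and spawns the initial tiles, calling DisplayHUD on each loop pass to create or reveal one widget.
; Each new tile attaches to the last one's transform, or StartPoint if first, and its exit event is bound to keep the path extending.
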(event `self.ReceiveBeginPlay`
  (bind _asbp_run_character (cast `/Game/Actors/BP_RunCharacter` (`GameplayStatics.GetPlayerCharacter` 0)))
  (bind _output_get (set `self.Player` _asbp_run_character))
  (add `/Game/Actors/BP_RunCharacter.OnPlayerDie` _output_get (`|CreateDelegate` :!event `OnPlayerDie`))
  (for _ (range (+ (`self.NumberOfInitialTiles`) 1))
    (`self.OnExitTile_Event` null)
    (`self.DisplayHUD`)))

(event `OnExitTile_Event`
  (params (Tile :type "/Game/Actors/BP_FloorTile Object Reference"))
  (bind _new_tile (`self.Spawn Next Tile`))
  (add `/Game/Actors/BP_FloorTile.OnExitTile` _new_tile (`|CreateDelegate` :!event `OnExitTile_Event`)))

(event `DisplayHUD`
  (bind _playerhud (`self.PlayerHUD`)
    (:`then`
      (`Widget.SetVisibility` _playerhud "Visible"))
    (:`else`
      (bind _returnvalue (`|CreateWidget` "/Game/Actors/W_PlayerHUD.W_PlayerHUD_C"))
      (set `/Game/Actors/W_PlayerHUD.GMRunCollectCoins` self _returnvalue)
      (bind _output_get (set `self.PlayerHUD` _returnvalue))
      (`UserWidget.AddToViewport` _output_get 0))))

(event `OnPlayerDie`
  (`KismetSystemLibrary.Delay` 3.0)
  (`KismetSystemLibrary.ExecuteConsoleCommand` " RestartLevel" null))

(fn `Spawn Next Tile`
  (returns (`New Tile` :type "/Game/Actors/BP_FloorTile Object Reference"))
  (locals (AttachPoint :type "Transform Structure"))
  (bind _tiles (`self.Tiles`))
  (if (`KismetArrayLibrary.Array_IsValidIndex` (`self.Tiles`))
    (bind _attachpoint (`/Game/Actors/BP_FloorTile.GetAttachTransform` (`|GetArrayItem` _tiles (`KismetArrayLibrary.Array_LastIndex` _tiles))))
    (set `local.AttachPoint` _attachpoint)
    (else
      (set `local.AttachPoint` (`self.StartPoint`))))
  (bind _returnvalue (`|SpawnActorFromClass` "/Game/Actors/BP_FloorTile.BP_FloorTile_C" (`local.AttachPoint`) "Undefined" "MultiplyWithRoot" null null))
  (`KismetArrayLibrary.Array_AddUnique` (`self.Tiles`) _returnvalue)
  (return _returnvalue))

(fn `UserConstructionScript`)